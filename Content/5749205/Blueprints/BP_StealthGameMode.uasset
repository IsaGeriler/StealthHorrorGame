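; BP_StealthGameMode is the stealth game's game mode, handling the lose and win end screens.
; HandlePlayerCaught and HandlePlayerEscaped each create a WBP_EndScreen for player 0, set a failure or escape message, and add it to the viewport.
; Both events then show the mouse cursor and switch to UI-only input.
; The file defines no callers for these events, and BeginPlay, Tick and the construction script are empty.
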(event `self.HandlePlayerCaught`
  (bind _returnvalue (`GameplayStatics.GetPlayerController` 0))
  (bind _caughtscreenref (`self.CaughtScreenRef`))
  (bind _returnvalue_2 (`|CreateWidget` "/Game/5749205/WBP_EndScreen.WBP_EndScreen_C" (`GameplayStatics.GetPlayerController` 0)))
  (set `self.CaughtScreenRef` _returnvalue_2)
  (`/Game/5749205/WBP_EndScreen.SetStatusText` _caughtscreenref "SIGNAL LOST!")
  (`UserWidget.AddToViewport` _caughtscreenref 0)
  (set `PlayerController.bShowMouseCursor` true _returnvalue)
  (`WidgetBlueprintLibrary.SetInputMode_UIOnlyEx` _returnvalue null))

(event `self.HandlePlayerEscaped`
  (bind _returnvalue (`GameplayStatics.GetPlayerController` 0))
  (bind _endscreenref (`self.EndScreenRef`))
  (bind _returnvalue_2 (`|CreateWidget` "/Game/5749205/WBP_EndScreen.WBP_EndScreen_C" (`GameplayStatics.GetPlayerController` 0)))
  (set `self.EndScreenRef` _returnvalue_2)
  (`/Game/5749205/WBP_EndScreen.SetStatusText` _endscreenref "YOU FOUND THE WAY OUT!")
  (`UserWidget.AddToViewport` _endscreenref 0)
  (set `PlayerController.bShowMouseCursor` true _returnvalue)
  (`WidgetBlueprintLibrary.SetInputMode_UIOnlyEx` _returnvalue null))

(fn `UserConstructionScript`)